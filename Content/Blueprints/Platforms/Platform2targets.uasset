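; Platform Blueprint that shuttles back and forth between the positions of two target actors, Target1 and Target2.
; On BeginPlay it caches both positions and snaps to the first, disabling movement if either target is invalid.
; Tick steps it by Velocity per frame, unscaled by delta time, applying the world-space direction as a local offset.
; It flips direction once within one step of the destination.
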(event `self.ReceiveBeginPlay`
  ;[1 0 0] BEGIN PLAY
  (`self.Set First Location`)
  (`self.Set Second Location`))

(event `Set Second Location`
  (bind _target2 (`self.Target2`))
  ;[0.7396 0.5345 0] Set second location
  (if (`KismetSystemLibrary.IsValid` _target2)
    (set `self.SecondPosition` (`SceneComponent.K2_GetComponentLocation` (`Actor.RootComponent` _target2)))
    (else
      (set `self.canMoove` false))))

(event `Set First Location`
  (bind _target1 (`self.Target1`))
  ;[0.7396 0.5345 0] Set first location
  (if (`KismetSystemLibrary.IsValid` _target1)
    (bind _output_get (set `self.FirstPosition` (`SceneComponent.K2_GetComponentLocation` (`Actor.RootComponent` _target1))))
    (`self.K2_SetActorLocation` _output_get)
    (else
      (set `self.canMoove` false))))

(event `self.ReceiveTick`
  (params (DeltaSeconds :type "Float (single-precision)"))
  ;[0.6302 0.3998 0] TICK
  (if (`self.canMoove`)
    (if (`self.ToFirst`)
      (`self.MoveToPosition` (`self.FirstPosition`))
      (else
        (`self.MoveToPosition` (`self.SecondPosition`))))))

(event `MoveToPosition`
  (params (Position :type "Vector Structure"))
  (bind _returnvalue (`self.K2_GetActorLocation`))
  (bind _velocity (`self.velocity`))
  ;[0.651 0.4528 0] MOVE TO POSITION
  (if (> (`KismetMathLibrary.VSize` (- _returnvalue Position)) _velocity)
    (`self.K2_AddActorLocalOffset` (* (`KismetMathLibrary.GetDirectionUnitVector` _returnvalue Position) _velocity))
    (else
      (set `self.ToFirst` (not (`self.ToFirst`))))))

(fn `UserConstructionScript`)